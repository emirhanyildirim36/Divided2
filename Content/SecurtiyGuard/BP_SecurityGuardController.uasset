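; AI controller for the security guard that detects the player and switches the guard between normal and chase movement.
; On possess it runs BT_SecurityGuard, and its AI Perception updates write the TargetActor and IsPlayerSeen blackboard keys for that tree.
; Sensing the first-person character raises the guard's walk speed, while losing it clears the target and lowers the speed again.
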(event `self.AIPerception.OnTargetPerceptionUpdated`
  (params (Actor :type "Actor Object Reference") (Stimulus :type "AIStimulus Structure"))
  (bind _returnvalue (`AIBlueprintHelperLibrary.GetBlackboard` null))
  (bind _asbp_first_person_character (cast `/Game/FirstPerson/Blueprints/BP_FirstPersonCharacter` Actor))
  (if (`.bSuccessfullySensed` (break `AIStimulus` Stimulus))
    (`BlackboardComponent.SetValueAsObject` _returnvalue "TargetActor" _asbp_first_person_character)
    (`BlackboardComponent.SetValueAsBool` _returnvalue "IsPlayerSeen" true)
    (bind _asbp_security_guard (cast `/Game/SecurtiyGuard/BP_SecurityGuard` (`self.K2_GetPawn`)))
    (set `CharacterMovementComponent.MaxWalkSpeed` 550.0 (`Character.CharacterMovement` _asbp_security_guard))
    (else
      (`BlackboardComponent.ClearValue` _returnvalue "TargetActor")
      (`BlackboardComponent.SetValueAsBool` _returnvalue "IsPlayerSeen" false)
      (bind _asbp_security_guard_2 (cast `/Game/SecurtiyGuard/BP_SecurityGuard` (`self.K2_GetPawn`)))
      (set `CharacterMovementComponent.MaxWalkSpeed` 300.0 (`Character.CharacterMovement` _asbp_security_guard_2)))))

(event `self.ReceivePossess`
  (params (PossessedPawn :type "Pawn Object Reference"))
  (`self.RunBehaviorTree` "/Game/SecurtiyGuard/BT_SecurityGuard.BT_SecurityGuard"))

(fn `UserConstructionScript`)