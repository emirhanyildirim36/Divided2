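; Password gate actor that shows a password screen while the player is at its trigger.
; When BP_FirstPersonCharacter enters the Tetik trigger, it creates and stores a WBD_Şifre widget, adds it to the viewport, shows the cursor and allows game and UI input.
; Any end overlap, with no actor check, removes the stored widget, hides the cursor and restores game-only input.
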(event `self.tetik.OnComponentBeginOverlap`
  (params (OverlappedComponent :type "PrimitiveComponent Object Reference") (OtherActor :type "Actor Object Reference") (OtherComp :type "PrimitiveComponent Object Reference") (OtherBodyIndex :type Integer) (bFromSweep :type Boolean) (SweepResult :type "HitResult Structure (by ref)"))
  (bind _returnvalue (`GameplayStatics.GetPlayerController` 0))
  (cast `/Game/FirstPerson/Blueprints/BP_FirstPersonCharacter` OtherActor)
  (bind _returnvalue_2 (`|CreateWidget` "/Game/WBD_Şifre.WBD_Şifre_C"))
  (set `self.açılanşifreekranı` _returnvalue_2)
  (`UserWidget.AddToViewport` _returnvalue_2 0)
  (set `PlayerController.bShowMouseCursor` true _returnvalue)
  (`WidgetBlueprintLibrary.SetInputMode_GameAndUIEx` _returnvalue null))

(event `self.tetik.OnComponentEndOverlap`
  (params (OverlappedComponent :type "PrimitiveComponent Object Reference") (OtherActor :type "Actor Object Reference") (OtherComp :type "PrimitiveComponent Object Reference") (OtherBodyIndex :type Integer))
  (bind _returnvalue (`GameplayStatics.GetPlayerController` 0))
  (`Widget.RemoveFromParent` (`self.açılanşifreekranı`))
  (set `PlayerController.bShowMouseCursor` false _returnvalue)
  (`WidgetBlueprintLibrary.SetInputMode_GameOnly` _returnvalue))

(fn `UserConstructionScript`)