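; BP_Tırmanma is an elevator that the player calls with the F key from inside a trigger volume.
; Overlapping Tetik enables input and shows the YazıF prompt, and leaving disables input and hides it, with no check on the overlapping actor.
; F plays the Asansörmotoru timeline, which lerps the static mesh's relative height upward.
; When the timeline finishes, a delay precedes reversing it to lower the mesh.
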(event `self.Tetik.OnComponentBeginOverlap`
  (params (OverlappedComponent :type "PrimitiveComponent Object Reference") (OtherActor :type "Actor Object Reference") (OtherComp :type "PrimitiveComponent Object Reference") (OtherBodyIndex :type Integer) (bFromSweep :type Boolean) (SweepResult :type "HitResult Structure (by ref)"))
  (`self.EnableInput` (`GameplayStatics.GetPlayerController` 0))
  (`SceneComponent.SetVisibility` (`self.Yazı F`) true false))

(event `Key|F`
  (params (Key :type "Key Structure"))
  (bind (_relativelocation_x _relativelocation_y) (`KismetMathLibrary.BreakVector` (`SceneComponent.RelativeLocation` (`self.StaticMesh`))))
  (:`Pressed`
    (bind (_direction `_yükseliş`) (`Timeline|asansörmotoru` :!via `PlayFromStart` :!label _label)
      (:`Update`
        (`SceneComponent.K2_SetRelativeLocation` (`self.StaticMesh`) (`KismetMathLibrary.MakeVector` _relativelocation_x _relativelocation_y (`KismetMathLibrary.Lerp` 0.0 600.0 `_yükseliş`)) false false))
      (:`Finished`
        (`KismetSystemLibrary.Delay` 4.0)
        (goto _label :!via `Reverse`)))))

(event `self.Tetik.OnComponentEndOverlap`
  (params (OverlappedComponent :type "PrimitiveComponent Object Reference") (OtherActor :type "Actor Object Reference") (OtherComp :type "PrimitiveComponent Object Reference") (OtherBodyIndex :type Integer))
  (`self.DisableInput` (`GameplayStatics.GetPlayerController` 0))
  (`SceneComponent.SetVisibility` (`self.Yazı F`) false false))

(fn `UserConstructionScript`)