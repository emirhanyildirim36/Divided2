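; BP_Ayna (mirror) is the finish trigger that ends a timed run in the first-person game.
; The first overlap on Tetik fires a DoOnce before the character cast; if it is the player, the final screen appears.
; It reads Time from WBP_PlayerUI, saves it to EniyiSüre in the BP_OyunHafızası game instance if lower, as the best time.
; After a short delay it opens Lvl_FirstPerson.
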(event `self.tetik.OnComponentBeginOverlap`
  (params (OverlappedComponent :type "PrimitiveComponent Object Reference") (OtherActor :type "Actor Object Reference") (OtherComp :type "PrimitiveComponent Object Reference") (OtherBodyIndex :type Integer) (bFromSweep :type Boolean) (SweepResult :type "HitResult Structure (by ref)"))
  (`/Engine/EditorBlueprintResources/StandardMacros.DoOnce` false
    (:`Completed`
      (cast `/Game/FirstPerson/Blueprints/BP_FirstPersonCharacter` OtherActor)
      (bind _returnvalue (`|CreateWidget` "/Game/UI/WBD_Final_Ekranı.WBD_Final_Ekranı_C"))
      (`UserWidget.AddToViewport` _returnvalue 0)
      (bind _foundwidgets (`WidgetBlueprintLibrary.GetAllWidgetsOfClass` "/Game/Can/UI/WBP_PlayerUI.WBP_PlayerUI_C"))
      (bind `_asbp_oyun_hafızası` (cast `/Game/BP_OyunHafızası` (`GameplayStatics.GetGameInstance`)))
      (bind _time (`/Game/Can/UI/WBP_PlayerUI.Time` (`|GetArrayItem` _foundwidgets)))
      (if (< _time (`/Game/BP_OyunHafızası.EniyiSüre` `_asbp_oyun_hafızası`))
        (set `/Game/BP_OyunHafızası.EniyiSüre` _time `_asbp_oyun_hafızası`))
      (`KismetSystemLibrary.Delay` 2.0)
      (`GameplayStatics.OpenLevel` "Lvl_FirstPerson"))))

(fn `UserConstructionScript`)